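; Base female survivor character Blueprint that sets up dynamic material instances for head, torso and legs on BeginPlay.
; Number keys act as apparent debug triggers for survivor states: attack, injured, dying, normal and hook go through Server-named events, while escaped and dead are called directly.
; Custom movement updates force a constant small X velocity.
; An unconnected leftover graph toggles collision and gravity.
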(event Custom|ServerSetSurvivorNormal
  (Class|SurvivorCharacter|SetSurvivorNormal))

(event Custom|ServerEvent
  (Class|SurvivorCharacter|AuthHookSurvivor))

(event Custom|ServerSetSurvivorDying
  (Class|SurvivorCharacter|SetSurvivorDying))

(event Custom|ServerSetSurvivorInjured
  (Class|SurvivorCharacter|SetSurvivorInjured))

(event Custom|ServerAttackSurvivor
  (Class|SurvivorCharacter|AttackSurvivor))

(event Custom|K2_UpdateCustomMovement_1
  (params (DeltaTime :type Float%20%28single-precision%29))
  (Variables|/Script/Engine.MovementComponent|SetVelocity (Variables|Character|GetCharacterMovement) "1.000000,0.000000,0.000000"))

(event EventBeginPlay
  (bind _mesh (Variables|Character|GetMesh))
  (Rendering|Material|CreateDynamicMaterialInstance _mesh 0 "/Game/Assets/JMS/Animation/MI_CMHead00.MI_CMHead00" "None" :!class /Script/Engine.PrimitiveComponent)
  (Rendering|Material|CreateDynamicMaterialInstance _mesh 1 "/Game/Assets/JMS/Animation/MI_CMTorso00.MI_CMTorso00" "None" :!class /Script/Engine.PrimitiveComponent)
  (Rendering|Material|CreateDynamicMaterialInstance _mesh 2 "/Game/Assets/JMS/Animation/MI_CMLegs00.MI_CMLegs00" "None" :!class /Script/Engine.PrimitiveComponent))

(event Collision|EventActorBeginOverlap
  (params (OtherActor :type Actor%20Object%20Reference)))

(event EventTick
  (params (DeltaSeconds :type Float%20%28single-precision%29)))

(event Input|KeyboardEvents|1
  (params (Key :type Key%20Structure :default "None"))
  (:Pressed
    (CallFunction|ServerAttackSurvivor)))

(event Input|KeyboardEvents|7
  (params (Key :type Key%20Structure :default "None"))
  (:Pressed
    (CallFunction|ServerEvent)))

(event Input|KeyboardEvents|3
  (params (Key :type Key%20Structure :default "None"))
  (:Pressed
    (CallFunction|ServerSetSurvivorDying)))

(event Input|KeyboardEvents|2
  (params (Key :type Key%20Structure :default "None"))
  (:Pressed
    (CallFunction|ServerSetSurvivorInjured)))

(event Input|KeyboardEvents|4
  (params (Key :type Key%20Structure :default "None"))
  (:Pressed
    (CallFunction|ServerSetSurvivorNormal)))

(event Input|KeyboardEvents|8
  (params (Key :type Key%20Structure :default "None"))
  (:Pressed
    (Class|SurvivorCharacter|SetSurvivorEscaped)))

(event Input|KeyboardEvents|9
  (params (Key :type Key%20Structure :default "None"))
  (:Pressed
    (Class|SurvivorCharacter|SetSurvivorDead)))

(fn ConstructionScript)