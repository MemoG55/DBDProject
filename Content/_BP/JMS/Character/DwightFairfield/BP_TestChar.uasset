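; BP_TestChar is a test character Blueprint in the DwightFairfield character folder for trying out animation and movement.
; Pressing 1 plays a stand-idle montage on the mesh and prints the returned value, and pressing W adds a forward force to the character movement.
; Unconnected leftover nodes hold experiments with mesh merging, a run montage, and leader-pose setup; BeginPlay, Tick and the construction script are empty.
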(event EventBeginPlay)

(event Collision|EventActorBeginOverlap
  (params (OtherActor :type Actor%20Object%20Reference)))

(event EventTick
  (params (DeltaSeconds :type Float%20%28single-precision%29)))

(event Input|KeyboardEvents|1
  (params (Key :type Key%20Structure))
  (:Pressed
    (bind _returnvalue (Animation|Montage|MontagePlay (Components|SkeletalMesh|GetAnimInstance (Variables|Character|GetMesh)) "/Game/_BP/JMS/Common/AnimMontage/DFAnimationRunAndIdle_Anim_Armature_M_StandIdle_Montage.DFAnimationRunAndIdle_Anim_Armature_M_StandIdle_Montage" 1.0 "MontageLength" 0.0 true))
    (Development|PrintString (Utilities|String|ToString(Float) _returnvalue))))

(event Input|KeyboardEvents|2
  (params (Key :type Key%20Structure)))

(event Input|KeyboardEvents|W
  (params (Key :type Key%20Structure))
  (:Pressed
    (Physics|AddForce (Variables|Character|GetCharacterMovement) (* (Transformation|GetActorForwardVector) 1e+03))))

(fn ConstructionScript)