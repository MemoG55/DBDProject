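; Game instance Blueprint that creates and joins online sessions through Advanced Sessions nodes.
; On Init, after a short delay, a dedicated server creates a LAN session with presence and lobbies off.
; CreateSession hosts a LAN session and server-travels to InGameLevel as a listen server.
; Accepted invites join the offered session, with results only printed to screen for debugging.
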(event Custom|CreateSession
  ;[1 1 1] Create Session
  (|AdvancedSession 0 (Game|GetPlayerController 0) 100 0 true true false true true true false false false true false true
    (:OnSuccess
      (Class|AdvancedSessionsLibrary|ServerTravel "/Game/_BP/Shared/Level/InGameLevel?listen" false false)
      (Development|PrintString "CreateSession::Success" true true "(R=1.000000,G=0.000000,B=0.073878,A=1.000000)"))
    (:OnFailure
      (Development|PrintString "CreateSession::Failed" true true "(R=0.000000,G=0.182344,B=1.000000,A=1.000000)"))))

(event EventOnSessionInviteAccepted
  (params (LocalPlayerNum :type Integer) (PersonInvited :type BP%20Unique%20Net%20Id%20Structure) (SessionToJoin :type Blueprint%20Session%20Result%20Structure%20%28by%20ref%29))
  ;[1 1 1] Join Session(via invite)
  (|JoinSession (Game|GetPlayerController 0) SessionToJoin
    (:then
      (Development|PrintString "Invite Accept Called"))
    (:OnSuccess
      (Development|PrintString "Invite Join Succeed"))
    (:OnFailure
      (Development|PrintString "Invite Join Failed"))))

(event EventInit
  (Utilities|FlowControl|Delay 1.0)
  (if (Networking|IsDedicatedServer)
    (|AdvancedSession 0 0 100 0 true true true false false false false false false true false true
      (:OnSuccess
        (Development|PrintString "CreateSessionComplete")))))