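; GA_BPExitDoor is the gameplay ability for the exit door object, built to advance interaction progress while interactors are present.
; Its GetActors event ticks the owner's interactable component, then ends the ability and clears the timer when no interactors remain or the ObjAbilitySystemComponent reports max task.
; The looping timer meant to poll GetActors is disconnected, and ActivateAbility is empty, so this graph never starts that loop.
; A TODO notes missing per-player-count checks.
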(event Custom|GetActors
  (bind _returnvalue (Class|ObjGameplayAbility|GetInteractableComponentfromActorInfo))
  (bind _returnvalue_2 (Class|ObjGameplayAbility|GetOwnerObjectfromActorInfo))
  (Utilities|IsValid _returnvalue
    (:Is%20Valid
      (bind _returnvalue_3 (Class|InteractableComponent|GetInteractors _returnvalue))
      (if (Utilities|Array|IsEmpty _returnvalue_3)
        ;[1 1 1] Attribute 변화 처리 TODO:: 인원별 체크 로직 추가
        (Utilities|Time|ClearandInvalidateTimerbyHandle (Variables|Default|GetTimer) :!label _label)
        (Ability|EndAbility)
        (else
          (Class|InteractableComponent|TickInteraction (Class|ObjGameplayAbility|GetInteractableComponentfromActorInfo) _returnvalue_2)
          (bind _asobj_ability_system_component (Utilities|Casting|CastToObjAbilitySystemComponent (Ability|GetAbilitySystemComponent _returnvalue_2)))
          (if (Class|ObjAbilitySystemComponent|IsMaxTask _asobj_ability_system_component)
            (goto _label)))))))

(event Ability|EventActivateAbility)

(event Ability|EventOnEndAbility
  (params (bWasCancelled :type Boolean)))