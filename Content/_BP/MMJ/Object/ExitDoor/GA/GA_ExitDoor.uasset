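; Gameplay ability for the exit door object that advances its task progress until completion.
; On activation, a looping timer fetches the door's interactors and applies the GEGenerator_Repair effect to the door's own ASC, even with no interactors.
; When the ObjAbilitySystemComponent reports max task, the timer clears and the ability ends, setting the door inactive.
; Per-interactor attribute checks are unfinished TODOs, so interactors do not affect progress.
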(event Custom|GetActors
  (bind _returnvalue (Class|ObjGameplayAbility|GetOwnerObjectfromActorInfo))
  (bind _returnvalue_2 (Class|ObjGameplayAbility|GetOwnerObjectfromActorInfo))
  (bind _returnvalue_3 (Ability|GetAbilitySystemComponent _returnvalue_2))
  (Utilities|IsValid _returnvalue
    (:Is%20Valid
      (bind _returnvalue_4 (Class|DBDObject|GetInteractors _returnvalue))
      (for _array_element _returnvalue_4
        ;[1 1 1] 인원 별 ASC가져와서 Attribute정보 체크 TODO :: PlayerState->ASC 추출방법확인
        (Utilities|IsValid (Ability|GetAbilitySystemComponent _array_element)))
      ;[1 1 1] Attribute 변화 처리 TODO:: 인원별 체크 로직 추가
      (GameplayEffects|ApplyGameplayEffectToSelf :self _returnvalue_3 :GameplayEffectClass "/Game/_BP/MMJ/Object/Generator/GE/GEGenerator_Repair.GEGenerator_Repair_C" :Level 1.0)
      (bind _asobj_ability_system_component (Utilities|Casting|CastToObjAbilitySystemComponent _returnvalue_3))
      (if (Class|ObjAbilitySystemComponent|IsMaxTask _asobj_ability_system_component)
        (Utilities|Time|ClearandInvalidateTimerbyHandle (Variables|Default|GetTimer))
        (Ability|EndAbility)))))

(event Ability|EventActivateAbility
  (bind _returnvalue (Utilities|Time|SetTimerbyEvent (delegate Custom|GetActors) 0.1 true))
  (Variables|Default|SetTimer _returnvalue))

(event Ability|EventOnEndAbility
  (params (bWasCancelled :type Boolean))
  (Class|DBDObject|SetIsActive (Class|ObjGameplayAbility|GetOwnerObjectfromActorInfo) false))