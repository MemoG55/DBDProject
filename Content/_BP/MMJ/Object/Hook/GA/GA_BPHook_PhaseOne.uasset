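; Gameplay Ability for the first phase of a hook object, driving its interaction progress while the ability is active.
; On activation a looping 0.1-second timer calls TickInteraction on the owner's interactable component while it has interactors.
; The timer clears and the ability ends when the object's ability system reports the current attribute at max, or when no interactors remain.
; OnEndAbility is empty, so only the tick clears the timer.
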(event Custom|TickTask
  (bind _returnvalue (Class|ObjGameplayAbility|GetOwnerObjectfromActorInfo))
  (bind _returnvalue_2 (Class|ObjGameplayAbility|GetInteractableComponentfromActorInfo))
  (Utilities|IsValid _returnvalue_2
    (:Is%20Valid
      (bind _returnvalue_3 (Class|InteractableComponent|GetInteractors _returnvalue_2))
      (if (Utilities|Array|IsNotEmpty _returnvalue_3)
        (Class|InteractableComponent|TickInteraction (Class|ObjGameplayAbility|GetInteractableComponentfromActorInfo) _returnvalue)
        (bind _asobj_ability_system_component (Utilities|Casting|CastToObjAbilitySystemComponent (Ability|GetAbilitySystemComponent _returnvalue)))
        (bind _returnvalue_4 (Class|ObjAbilitySystemComponent|IsMaxAttribute _asobj_ability_system_component (Variables|Default|GetMax%20Attribute) (Variables|Default|GetCurrent%20Attribute)))
        (if _returnvalue_4
          (Utilities|Time|ClearandInvalidateTimerbyHandle (Variables|Default|GetTimer) :!label _label)
          (Ability|EndAbility))
        (else
          (goto _label))))))

(event Ability|EventActivateAbility
  (Utilities|IsValid (Class|ObjGameplayAbility|GetOwnerObjectfromActorInfo)
    (:Is%20Valid
      (bind _returnvalue (Utilities|Time|SetTimerbyEvent (delegate Custom|TickTask) 0.1 true))
      (Variables|Default|SetTimer _returnvalue))))

(event Ability|EventOnEndAbility
  (params (bWasCancelled :type Boolean)))