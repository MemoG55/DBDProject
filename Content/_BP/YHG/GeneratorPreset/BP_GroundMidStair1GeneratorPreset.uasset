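; Preset actor, named for a ground mid-stair location, that pairs a generator with lamp pole lighting that turns on when the generator completes.
; BeginPlay casts its child actor to BP_Generator and binds to that generator's interactable component OnComplete.
; On completion it activates the light locally and calls a Client event to repeat it, raising the lamp pole material's brightness and showing four spotlights.
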(event Custom|OnComplete_Event
  (CallFunction|ActivateGeneratorLight)
  (CallFunction|ClientActivateGeneratorLight))

(event Custom|Client_ActivateGeneratorLight
  (CallFunction|ActivateGeneratorLight))

(event EventBeginPlay
  (bind _asbp_generator (CallFunction|RegisterGenerator))
  (bind _output_get (Variables|Default|SetAs%20BP%20Generator _asbp_generator))
  (Utilities|IsValid _output_get
    (:Is%20Valid
      (EventDispatchers|AssignOnComplete (Class|DBDObject|GetInteractableComponent _output_get) (delegate Custom|OnComplete_Event)))))

(event Collision|EventActorBeginOverlap
  (params (OtherActor :type Actor%20Object%20Reference)))

(event EventTick
  (params (DeltaSeconds :type Float%20%28single-precision%29)))

(fn ConstructionScript)

(fn RegisterGenerator
  (bind _asbp_generator (Utilities|Casting|CastToBP_Generator (Variables|/Script/Engine.ChildActorComponent|GetChildActor (Variables|Default|GetBP_Generator))))
  (return _asbp_generator))

(fn ActivateGeneratorLight
  (Rendering|Material|SetScalarParameterValueonMaterials (Variables|Default|GetGeneratorLampPoles_SM_LampPole) "Brightness" 4.0)
  (Rendering|SetVisibility (Variables|Default|GetSpotLight) true false))