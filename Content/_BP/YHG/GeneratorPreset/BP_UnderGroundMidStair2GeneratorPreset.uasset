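; Preset actor for the underground mid-stair area that pairs a generator with a sliding door and lamp.
; On BeginPlay it binds to the generator's interactable completion and caches the moving door component through nested child-actor casts.
; Completion plays the door animation, brightens the lamp material and shows the spotlight, then calls a client-named event that repeats those effects, apparently for networked clients.
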(event Custom|OnComplete_Event
  (CallFunction|PlayMovingSlidingDoor)
  (CallFunction|ActivateGeneratorLight)
  (CallFunction|ClientOpenSlidingDoor))

(event Custom|Client_OpenSlidingDoor
  (CallFunction|PlayMovingSlidingDoor)
  (CallFunction|ActivateGeneratorLight))

(event EventBeginPlay
  (bind _asbp_generator (CallFunction|RegisterGenerator))
  (bind _output_get (Variables|Default|SetAs%20BP%20Generator _asbp_generator))
  (Utilities|IsValid _output_get
    (:Is%20Valid
      (EventDispatchers|AssignOnComplete (Class|DBDObject|GetInteractableComponent _output_get) (delegate Custom|OnComplete_Event))
      (bind _finland_sliding_door_1 (CallFunction|RegisterMovingSlidingDoor))
      (Variables|Default|SetFinland%20Sliding%20Door%201 _finland_sliding_door_1))))

(event Collision|EventActorBeginOverlap
  (params (OtherActor :type Actor%20Object%20Reference)))

(event EventTick
  (params (DeltaSeconds :type Float%20%28single-precision%29)))

(fn ConstructionScript)

(fn RegisterMovingSlidingDoor
  (bind _asbp_sliding_door_2 (Utilities|Casting|CastToBP_SlidingDoor2 (Variables|/Script/Engine.ChildActorComponent|GetChildActor (Variables|Default|GetBP_SlidingDoor2))))
  (bind _asbp_sliding_door_1 (Utilities|Casting|CastToBP_SlidingDoor1 (Variables|/Script/Engine.ChildActorComponent|GetChildActor (Variables|/Game/Assets/YHG/Map/Finland/Structure/Sub/SlidingDoor/BP_SlidingDoor2.BP_SlidingDoor2_C|GetBP_SlidingDoor1 _asbp_sliding_door_2))))
  (return (Variables|/Game/Assets/YHG/Map/Finland/Structure/Sub/SlidingDoor/BP_SlidingDoor1.BP_SlidingDoor1_C|GetFinland_SlidingDoor1 _asbp_sliding_door_1)))

(fn PlayMovingSlidingDoor
  (bind _finland_sliding_door_1 (Variables|Default|GetFinland%20Sliding%20Door%201))
  (Utilities|IsValid _finland_sliding_door_1
    (:Is%20Valid
      (Audio|Components|Audio|Play _finland_sliding_door_1 false))))

(fn RegisterGenerator
  (bind _asbp_generator (Utilities|Casting|CastToBP_Generator (Variables|/Script/Engine.ChildActorComponent|GetChildActor (Variables|Default|GetBP_Generator))))
  (return _asbp_generator))

(fn ActivateGeneratorLight
  (Rendering|Material|SetScalarParameterValueonMaterials (Variables|Default|GetGeneratorLampPoles_SM_Generator_SmallPole) "Brightness" 4.0)
  (Rendering|SetVisibility (Variables|Default|GetSpotLight) true false))